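; BP_BrownGlass is a placed item that drops antigen when it lands on a BloodGlass.
; It resolves on its first Tick with an overlap test against the BloodGlass found by GetActorOfClass.
; On overlap it calls DropAntigen on that glass; otherwise it returns itself to the Player's inventory and plays a failure sound.
; Either branch destroys the actor, so it acts as a one-shot use check.
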(event `self.ReceiveTick`
  (params (DeltaSeconds :type "Float (single-precision)"))
  (bind _returnvalue (`GameplayStatics.GetActorOfClass` "/Game/FST/YH/Assets/StarterContent/Assets/Room3/BloodGlass/BloodGlass.BloodGlass_C"))
  (if (`self.IsOverlappingActor` _returnvalue)
    (`/Game/FST/YH/Assets/StarterContent/Assets/Room3/BloodGlass/BloodGlass.DropAntigen` _returnvalue)
    (`self.K2_DestroyActor`)
    (else
      (bind _returnvalue_2 (`GameplayStatics.GetActorOfClass` "/Game/Character/Player.Player_C"))
      (`/Game/Character/Player.Add Item to Inventory` _returnvalue_2 "BP_BrownGlass_C")
      (`GameplayStatics.PlaySound2D` "/Game/FST/JE/Sound/무언가실패했을때.무언가실패했을때" 1.0 1.0 0.0 null null)
      (`self.K2_DestroyActor`))))

(fn `UserConstructionScript`
  (`parent.UserConstructionScript`))