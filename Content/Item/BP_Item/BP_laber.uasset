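; BP_laber is an item actor, apparently a lever, that resolves its use against the TM_Panel as soon as it ticks.
; If it overlaps the panel found in the level, it calls the panel's Laber function, plays a success sound at its location and destroys itself.
; Otherwise it adds BP_laber back to the Player's inventory, plays a failure sound and destroys itself.
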(event `self.ReceiveTick`
  (params (DeltaSeconds :type "Float (single-precision)"))
  (bind _returnvalue (`GameplayStatics.GetActorOfClass` "/Game/TM_Panel.TM_Panel_C"))
  (if (`self.IsOverlappingActor` _returnvalue)
    (`/Game/TM_Panel.Laber` _returnvalue)
    (`GameplayStatics.PlaySoundAtLocation` "/Game/FST/JE/Sound/상호작용_맞을때.상호작용_맞을때" (`self.K2_GetActorLocation`) (struct) 1.0 1.0 0.0 null null null)
    (`self.K2_DestroyActor`)
    (else
      (bind _returnvalue_2 (`GameplayStatics.GetActorOfClass` "/Game/Character/Player.Player_C"))
      (`/Game/Character/Player.Add Item to Inventory` _returnvalue_2 "BP_laber_C")
      (`GameplayStatics.PlaySound2D` "/Game/FST/JE/Sound/무언가실패했을때.무언가실패했을때" 1.0 1.0 0.0 null null)
      (`self.K2_DestroyActor`))))

(fn `UserConstructionScript`
  (`parent.UserConstructionScript`))